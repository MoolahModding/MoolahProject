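; Spawn group actor for map units that creates and tracks a set of BP_SpawnPawn markers for either civilians or cops.
; The SpawnPawns event spawns markers at the static mesh's relative transform, attaches them and adds them to PawnSpawnArray.
; A separate SpawnPawns function spawns owned, unattached markers at the actor's transform.
; The construction script applies civilian or cop materials to the tracked markers' meshes based on IsEnabledForCivilians.
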(event `Spawn Pawns`
  (for _ (range (`self.Spawn Pawn Amount`))
    (bind _returnvalue (`|SpawnActorFromClass` "/Game/Mods/MapUnits/Blueprints/BP_SpawnPawn.BP_SpawnPawn_C" (`SceneComponent.GetRelativeTransform` (`self.StaticMesh`)) "Undefined" "OverrideRootScale" null null))
    (`self.K2_AttachToActor` _returnvalue self "None" "KeepRelative" "KeepRelative" "KeepRelative" true)
    (`KismetArrayLibrary.Array_Add` (`self.PawnSpawnArray`) _returnvalue)))

(fn `SpawnPawns`
  (params (`Amount of spawn pawns` :type Integer))
  (bind _array (`|MakeArray` null :!type "/Game/Mods/MapUnits/Blueprints/BP_SpawnPawn Object Reference"))
  (for _ (range `Amount of spawn pawns`)
    (bind _returnvalue (`|SpawnActorFromClass` "/Game/Mods/MapUnits/Blueprints/BP_SpawnPawn.BP_SpawnPawn_C" (`self.GetTransform` self) "Undefined" "OverrideRootScale" self null))
    (`KismetArrayLibrary.Array_Add` _array _returnvalue)
    (set `self.PawnSpawnArray` _array)))

(fn `UserConstructionScript`
  (if (`self.bIsEnabledForCivilians`)
    (for _array_element (`self.PawnSpawnArray`)
      (for _array_element_2 (`self.K2_GetComponentsByClass` _array_element "/Script/Engine.StaticMeshComponent")
        (`PrimitiveComponent.SetMaterial` _array_element_2 0 "/Game/Mods/MapUnits/Materials/MI_PawnSpawnCiv.MI_PawnSpawnCiv")))
    (else
      (for _array_element_3 (`self.PawnSpawnArray`)
        (for _array_element_4 (`self.K2_GetComponentsByClass` _array_element_3 "/Script/Engine.StaticMeshComponent")
          (`PrimitiveComponent.SetMaterial` _array_element_4 0 "/Game/Mods/MapUnits/Materials/MI_PawnSpawnCop.MI_PawnSpawnCop"))))))
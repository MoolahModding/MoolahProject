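; BP_SpawnPawnCiv is a map unit actor that marks a single pawn spawn point, apparently for civilians.
; Its construction script copies the static mesh's world location into WeightedLocation and builds one SBZ pawn spawn definition from the mesh's world transform, with no type name and a zero seed.
; The event graph is empty, and an unwired loop over attached BP_SpawnPawn actors never runs.
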(fn `UserConstructionScript`
  (set `self.WeightedLocation` (`SceneComponent.K2_GetComponentLocation` (`self.StaticMesh`)))
  (set `self.SpawnDefinitionArray` (`|MakeArray` (make `SBZPawnSpawnDefinition` (`SceneComponent.K2_GetComponentToWorld` (`self.StaticMesh`)))))
  (set `self.Seed` 0))